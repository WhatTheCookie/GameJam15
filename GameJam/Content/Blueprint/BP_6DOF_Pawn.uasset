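; BP_6DOF_Pawn is a ship pawn with six-degrees-of-freedom flight controls driven by input axes.
; LookUp, Turn and Roll apply local actor rotation directly from the axis values.
; MoveForward, MoveRight and Float set BodyMesh physics linear velocity along the actor's axes, scaled by ShipSpeed.
; Forward and right movement add to the current velocity, while Float replaces it.
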(event `InputAxis|LookUp`
  (params (AxisValue :type "Float (single-precision)"))
  ;[1 1 1] Mouse Movement
  (`self.K2_AddActorLocalRotation` (`KismetMathLibrary.MakeRotator` 0.0 AxisValue)))

(event `InputAxis|Roll`
  (params (AxisValue :type "Float (single-precision)"))
  ;[1 1 1] Mouse Movement
  (`self.K2_AddActorLocalRotation` (`KismetMathLibrary.MakeRotator` AxisValue)))

(event `InputAxis|Turn`
  (params (AxisValue :type "Float (single-precision)"))
  ;[1 1 1] Mouse Movement
  (`self.K2_AddActorLocalRotation` (`KismetMathLibrary.MakeRotator` 0.0 0.0 AxisValue)))

(event `InputAxis|MoveForward`
  (params (AxisValue :type "Float (single-precision)"))
  ;[1 1 1] Keyboard Movement
  (`|ExecutionSequence`
    (:`then_1`
      (`PrimitiveComponent.SetPhysicsLinearVelocity` (`self.BodyMesh`) (* (`KismetMathLibrary.GetForwardVector` (`self.K2_GetActorRotation`)) (* AxisValue (`self.shipSpeed`))) true "None"))))

(event `InputAxis|Float`
  (params (AxisValue :type "Float (single-precision)"))
  ;[1 1 1] Keyboard Movement
  (`PrimitiveComponent.SetPhysicsLinearVelocity` (`self.BodyMesh`) (* (`KismetMathLibrary.GetUpVector` (`self.K2_GetActorRotation`)) (* AxisValue (`self.shipSpeed`))) false "None"))

(event `InputAxis|MoveRight`
  (params (AxisValue :type "Float (single-precision)"))
  ;[1 1 1] Keyboard Movement
  (`PrimitiveComponent.SetPhysicsLinearVelocity` (`self.BodyMesh`) (* (`KismetMathLibrary.GetRightVector` (`self.K2_GetActorRotation`)) (* AxisValue (`self.shipSpeed`))) true "None"))

(fn `UserConstructionScript`)